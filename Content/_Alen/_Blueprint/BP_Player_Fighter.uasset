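; Player fighter jet pawn that rolls along the ground (e.g. launch pads) and takes off into free flight.
; On the ground, smoothed forward input creeps the jet forward and look input turns the camera; Space at enough forward input sets Flying and enables camera lag.
; In flight, forward input adjusts a clamped target thrust, AddFlightMode moves the jet each tick with swept offsets, and look/turn inputs drive interpolated pitch and roll.
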(event `self.ReceiveBeginPlay`
  ;[0 0 0] Event Begin Play
  (`|ExecutionSequence`
    (:`then_0`
      ;;[0.4167 0.4167 0.4167] When Take off, should go minimum set speed
      (set `self.TargetThrustSpeed` (`self.MinimumThrustSpeed`)))))

(event `self.ReceiveTick`
  (params (DeltaSeconds :type "Float (single-precision)"))
  ;[0 0 0] Event Tick
  (`|ExecutionSequence`
    (:`then_0`
      ;;[1 1 1] For Ground Movement. Interp value set to low value as fighter should speed up very gradually when grounded
      (bind _output_get (set `self.MoveForward Interp` (`KismetMathLibrary.FClamp` (`KismetMathLibrary.FInterpTo` (stale _output_get) (`self.GetInputAxisValue`) (`GameplayStatics.GetWorldDeltaSeconds`) 200.0) 0.0 1.0))))
    (:`then_1`
      ;[0 0 0] If Flying
      (if (`self.Flying?`)
        (`self.AddFlightMode`)))))

(event `InputAxis|Move Forward`
  (params (AxisValue :type "Float (single-precision)"))
  (bind _springarm (`self.SpringArm`))
  ;[0 0 0] If Flying W/S Increase and decreese speed
  (if (`self.Flying?`)
    (set `self.TargetThrustSpeed` (`KismetMathLibrary.FClamp` (+ (* AxisValue (`GameplayStatics.GetWorldDeltaSeconds`) 1500.0) (`self.TargetThrustSpeed`)) (`self.MinimumThrustSpeed`) (`self.MaximumThrustSpeed`))))
  (if (not (`self.Flying?`))
    (`|ExecutionSequence`
      (:`then_0`
        (`self.K2_AddActorWorldOffset` (`KismetMathLibrary.MakeVector` (.x (* (`self.GetActorForwardVector`) (`self.MoveForward Interp`) (/ (`self.TargetThrustSpeed`) 500.0))) (.y (* (`self.GetActorForwardVector`) (`self.MoveForward Interp`) (/ (`self.TargetThrustSpeed`) 500.0)))) true)
        ;[0 0 0] Set Jet to flying and add the camera lags
        (if (and (> (`self.MoveForward Interp`) 0.7) (`PlayerController.IsInputKeyDown` (`GameplayStatics.GetPlayerController` 0) "SpaceBar"))
          (set `self.Flying?` true)
          (bind _output_get (set `SpringArmComponent.bEnableCameraLag` true _springarm))
          (set `SpringArmComponent.bEnableCameraRotationLag` _output_get _springarm)
          (set `SpringArmComponent.bUsePawnControlRotation` false _springarm)
          (`self.K2_AddActorWorldOffset` (0.0 0.0 25.0) true))))))

(event `InputAxis|Look Up`
  (params (AxisValue :type "Float (single-precision)"))
  (bind _returnvalue (`GameplayStatics.GetWorldDeltaSeconds`))
  (bind _returnvalue_2 (* AxisValue (`KismetMathLibrary.SelectFloat` -1.0 1.0 (`self.InvertVecticle Flight?`))))
  ;[0 0 0] Look Up Input. if not flying add camera rotation. if flying add rotation to fighter
  (if (`self.Flying?`)
    (bind _output_get (set `self.FlightPitch` (`KismetMathLibrary.FInterpTo` (stale _output_get) _returnvalue_2 _returnvalue)))
    (`self.K2_AddActorLocalRotation` (`KismetMathLibrary.MakeRotator` 0.0 (* _output_get _returnvalue (`self.FlightTurnRate`))))
    (else
      (`self.AddControllerPitchInput` _returnvalue_2))))

(event `InputAxis|Turn`
  (params (AxisValue :type "Float (single-precision)"))
  (bind _returnvalue (`GameplayStatics.GetWorldDeltaSeconds`))
  ;[0 0 0] Turn Input
  (if (`self.Flying?`)
    (bind _output_get (set `self.FlightTurn` (`KismetMathLibrary.FInterpTo` (stale _output_get) AxisValue _returnvalue)))
    (`self.K2_AddActorLocalRotation` (`KismetMathLibrary.MakeRotator` (* _output_get _returnvalue (`self.FlightTurnRate`))))
    (else
      (`self.AddControllerYawInput` AxisValue))))

(fn `AddFlightMode`
  (bind _returnvalue (`GameplayStatics.GetWorldDeltaSeconds`))
  ;[0 0 0] Set Flight Speed
  (bind _output_get (set `self.CurrentThrustSpeed` (`KismetMathLibrary.FInterpTo` (stale _output_get) (`self.TargetThrustSpeed`) _returnvalue 8.0)))
  ;[0 0 0] Add Movement in forward direction
  (`self.K2_AddActorWorldOffset` (* (`SceneComponent.GetForwardVector` (`self.Box`)) (* _output_get _returnvalue)) true))

(fn `UserConstructionScript`)